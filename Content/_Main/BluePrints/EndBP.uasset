(event `self.Box.OnComponentBeginOverlap`
  (params (OverlappedComponent :type "PrimitiveComponent Object Reference") (OtherActor :type "Actor Object Reference") (OtherComp :type "PrimitiveComponent Object Reference") (OtherBodyIndex :type Integer) (bFromSweep :type Boolean) (SweepResult :type "HitResult Structure (by ref)"))
  (bind _asbp_first_person_character (cast `/Game/_Main/BluePrints/BP_FirstPersonCharacter` OtherActor))
  (`GameplayStatics.PlaySound2D` "/Game/Audio/WomanScream.WomanScream" 1.0 1.0 0.0 null null)
  (`SceneComponent.SetVisibility` (`/Game/_Main/BluePrints/BP_FirstPersonCharacter.Zombie` _asbp_first_person_character) true false)
  (`SceneComponent.SetVisibility` (`/Game/_Main/BluePrints/BP_FirstPersonCharacter.FirstPersonMesh` _asbp_first_person_character) false false)
  (`SceneComponent.SetVisibility` (`/Game/_Main/BluePrints/BP_FirstPersonCharacter.PistolMesh` _asbp_first_person_character) false false)
  (set `/Game/_Main/BluePrints/BP_FirstPersonCharacter.FinishedGame?` true _asbp_first_person_character)
  (`KismetSystemLibrary.Delay` 2.5)
  (`/Game/_Main/Widgets/MainWidget_W.ShowThanksWin` (`/Game/_Main/BluePrints/BP_FirstPersonCharacter.MainWidget` _asbp_first_person_character))
  (`KismetSystemLibrary.Delay` 1.5)
  (`GameplayStatics.OpenLevel` "MainMenu"))

(fn `UserConstructionScript`)