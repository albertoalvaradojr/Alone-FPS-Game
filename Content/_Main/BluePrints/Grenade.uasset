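; Thrown grenade actor that launches along the player's aim on spawn and explodes after a short fuse.
; BeginPlay applies an impulse from the controller's rotation, waits, then spawns an explosion emitter attached to the grenade and a sound at its location.
; A sphere overlap query then makes both zombie types drop ammo and destroys them, while ghosts receive GrenadeHit damage.
; The grenade destroys itself after a further delay.
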(event `self.ReceiveBeginPlay`
  (bind _grenade (`self.Grenade`))
  (`PrimitiveComponent.AddImpulse` (`self.Grenade`) (* (`KismetMathLibrary.Conv_RotatorToVector` (`Controller.GetControlRotation` (`GameplayStatics.GetPlayerController` 0))) (3000.0 3000.0 3000.0)) "None" false)
  (`KismetSystemLibrary.Delay` 1.0)
  (`GameplayStatics.SpawnEmitterAttached` "/Game/Realistic_Starter_VFX_Pack_Vol2/Particles/Explosion/P_Explosion_Big_B.P_Explosion_Big_B" _grenade)
  (`GameplayStatics.SpawnSoundAtLocation` "/Game/MilitaryWeapDark/Sound/GrenadeLauncher/GrenadeLauncher_Explosion_Cue.GrenadeLauncher_Explosion_Cue" (`SceneComponent.K2_GetComponentLocation` _grenade) (struct) 1.0 1.0 0.0 null null)
  (`|ExecutionSequence`
    (:`then_0`
      (for _array_element (`PrimitiveComponent.GetOverlappingActors` (`self.Sphere`) "/Game/_Main/Enemies/Zombie_BP.Zombie_BP_C")
        (bind _aszombie_bp (cast `/Game/_Main/Enemies/Zombie_BP` _array_element))
        (`/Game/_Main/Enemies/Zombie_BP.DropAmmo` _aszombie_bp)
        (`self.K2_DestroyActor` _array_element)))
    (:`then_1`
      (for _array_element_2 (`PrimitiveComponent.GetOverlappingActors` (`self.Sphere`) "/Game/_Main/Enemies/ZombieM_BP.ZombieM_BP_C")
        (bind _aszombie_m_bp (cast `/Game/_Main/Enemies/ZombieM_BP` _array_element_2))
        (`/Game/_Main/Enemies/ZombieM_BP.DropAmmo` _aszombie_m_bp)
        (`self.K2_DestroyActor` _array_element_2)))
    (:`then_2`
      (for _array_element_3 (`PrimitiveComponent.GetOverlappingActors` (`self.Sphere`) "/Game/_Main/Enemies/Ghost_BP.Ghost_BP_C")
        (bind _asghost_bp (cast `/Game/_Main/Enemies/Ghost_BP` _array_element_3))
        (`/Game/_Main/Enemies/Ghost_BP.GrenadeHit` _asghost_bp 50.0))
      (`KismetSystemLibrary.Delay` 2.0)
      (`self.K2_DestroyActor`))))

(fn `UserConstructionScript`)