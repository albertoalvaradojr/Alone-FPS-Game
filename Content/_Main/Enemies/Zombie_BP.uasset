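; Zombie enemy that chases the player from BeginPlay and raises its walk speed on seeing a pawn.
; It loops AI MoveTo into an attack montage whose notify applies damage through a sphere overlap at an arrow.
; Point damage plays hit reactions until health runs out, then it dies, fades horde audio, drops ammo and destroys itself.
; Random patrol and wave-mode kill reporting are left unwired.
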(event `self.ReceiveBeginPlay`
  (`self.RunTOPlayer`))

(event `self.ReceiveTick`
  (params (DeltaSeconds :type "Float (single-precision)"))
  ;[1 1 1] Patrolling
)

(event `self.PawnSensing.OnSeePawn`
  (params (Pawn :type "Pawn Object Reference"))
  ;[1 1 1] Sensing
  (set `CharacterMovementComponent.MaxWalkSpeed` 360.0 (`self.CharacterMovement`))
  (set `self.FoundPlayer?` true))

(event `RunTOPlayer`
  ;[0.2652 1 0.2584] Move ToPlayer
  (if (not (`self.IsDead?`))
    (`|AIMoveTo` self (0.0 0.0 0.0) (`GameplayStatics.GetPlayerCharacter` 0) 40.0
      (:`OnSuccess`
        (`self.AttackPlayer`))
      (:`OnFail`
        (`self.RunTOPlayer`)))))

(event `AttackPlayer`
  ;[1 1 1] Attack
  (`|PlayMontage` (`self.Mesh`) "/Game/_Main/Enemies/Zombie/Animations/zombie_attack_Montage1.zombie_attack_Montage1"
    (:`OnCompleted`
      (`self.RunTOPlayer`))
    (:`OnNotifyBegin`
      (`GameplayStatics.PlaySoundAtLocation` "/Game/_Main/Enemies/Zombie/Audio/AttackCue.AttackCue" (`self.K2_GetActorLocation`) (struct) 1.0 1.0 0.0 "/Game/MilitaryWeapDark/Sound/Attenuation/WeaponShot_att.WeaponShot_att" null null null)
      (bind (_outactors _returnvalue) (`KismetSystemLibrary.SphereOverlapActors` (`SceneComponent.K2_GetComponentLocation` (`self.Arrow1`)) 80.0 (`|MakeArray` "ObjectTypeQuery3" :!type "EObjectTypeQuery Enum") "/Game/_Main/BluePrints/BP_FirstPersonCharacter.BP_FirstPersonCharacter_C" (`|MakeArray` self :!type "Actor Object Reference")))
      (if _returnvalue
        (for _array_element _outactors
          (`GameplayStatics.ApplyDamage` _array_element 20.0 (`self.GetController`) self "/Script/Engine.DamageType"))))))

(event `self.ReceivePointDamage`
  (params (Damage :type "Float (single-precision)") (DamageType :type "DamageType Object Reference") (HitLocation :type "Vector Structure") (HitNormal :type "Vector Structure") (HitComponent :type "PrimitiveComponent Object Reference") (BoneName :type Name) (ShotFromDirection :type "Vector Structure") (InstigatedBy :type "Controller Object Reference") (DamageCauser :type "Actor Object Reference") (HitInfo :type "HitResult Structure (by ref)"))
  ;[1 1 1] Take Damage
  (if (`self.IsDead?`)
    _
    (elif (<= (`self.Health`) 0.0)
      (`self.Death` :!label _label)
      (else
        (bind _output_get (set `self.Health` (- (`self.Health`) Damage)))
        (if (<= _output_get 0.0)
          (goto _label)
          (else
            (`|PlayMontage` (`self.Mesh`) "/Game/_Main/Enemies/Zombie/Animations/Zombie_Reaction_Hit_mixamo_com_Montage.Zombie_Reaction_Hit_mixamo_com_Montage"
              (:`OnCompleted`
                (`self.RunTOPlayer`)))))))))

(event `Death`
  ;[0.5208 0.004563 0] Death
  (set `self.IsDead?` true)
  (`MovementComponent.StopMovementImmediately` (`self.CharacterMovement`))
  (`|PlayMontage` (`self.Mesh`) "/Game/_Main/Enemies/Zombie/Animations/zombie_dying_Montage.zombie_dying_Montage"
    (:`then`
      (`PrimitiveComponent.SetCollisionResponseToChannel` (`self.CapsuleComponent`) "ECC_Pawn" "ECR_Overlap")
      (`PrimitiveComponent.SetCollisionEnabled` (`self.Mesh`) "NoCollision")
      (`AudioComponent.AdjustVolume` (`self.hoarde`) 2.0 0.0 "Linear")
      (`KismetSystemLibrary.Delay` 4.0)
      (`self.DropAmmo`)
      (`self.K2_DestroyActor`))))

(event `DropAmmo`
  ;[0.4071 1 0.3711] Drop Ammo
  (`|SpawnActorFromClass` "/Game/_Main/BluePrints/AmmoPickUp.AmmoPickUp_C" (`KismetMathLibrary.MakeTransform` (`self.K2_GetActorLocation`)) "Undefined" "OverrideRootScale" null null))

(fn `UserConstructionScript`)