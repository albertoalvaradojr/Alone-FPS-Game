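; Showcase Blueprint for the M1A1 Abrams tank that exposes its adjustable features through generic slider, button and checkbox events.
; Each event forwards its value to a named setter for speed, skin, damaged model, turret rotation, firing, gun elevation, hatches or light emissivity.
; The setters are not defined in this graph, and the construction script only calls the parent's.
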(event `/Game/VigilanteContent/Shared/Showcase/Interfaces/BP_ShowcaseControlsInterface.SetSliderVariable0`
  (params (NewValue :type "Float (single-precision)"))
  ;[1 1 1] Speed
  (`self.SetSpeed` NewValue))

(event `/Game/VigilanteContent/Shared/Showcase/Interfaces/BP_ShowcaseControlsInterface.SetButtonsVariable0`
  (params (NewIndex :type Integer))
  ;[1 1 1] Skin variant
  (`self.SetSkinType` (`KismetMathLibrary.Conv_IntToDouble` NewIndex)))

(event `/Game/VigilanteContent/Shared/Showcase/Interfaces/BP_ShowcaseControlsInterface.SetCheckboxVariable0`
  (params (NewState :type Boolean))
  ;[1 1 1] Damaged model visibility
  (`self.SetShowDamaged` NewState))

(event `/Game/VigilanteContent/Shared/Showcase/Interfaces/BP_ShowcaseControlsInterface.SetSliderVariable1`
  (params (NewValue :type "Float (single-precision)"))
  ;[1 1 1] Turret Rotation
  (`self.SetTurretRotation` NewValue))

(event `/Game/VigilanteContent/Shared/Showcase/Interfaces/BP_ShowcaseControlsInterface.SetCheckboxVariable1`
  (params (NewState :type Boolean))
  ;[1 1 1] Firing activation
  (`self.SetFiringActive` NewState))

(event `/Game/VigilanteContent/Shared/Showcase/Interfaces/BP_ShowcaseControlsInterface.SetSliderVariable2`
  (params (NewValue :type "Float (single-precision)"))
  ;[1 1 1] Gun Elevation
  (`self.SetGunElevation` NewValue))

(event `/Game/VigilanteContent/Shared/Showcase/Interfaces/BP_ShowcaseControlsInterface.SetSliderVariable3`
  (params (NewValue :type "Float (single-precision)"))
  ;[1 1 1] Hatch Angle
  (`self.SetHatchesAngle` NewValue))

(event `/Game/VigilanteContent/Shared/Showcase/Interfaces/BP_ShowcaseControlsInterface.SetSliderVariable4`
  (params (NewValue :type "Float (single-precision)"))
  ;[1 1 1] Light emissivity
  (`self.SetLightsEmissivity` NewValue))

(fn `UserConstructionScript`
  (`parent.UserConstructionScript`))